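; PhysicsReset is a component that returns its owning actor to its starting state when the game restarts.
; On BeginPlay it saves the owner's transform and binds to the OnGameRestart dispatcher on BP_BreadGameState.
; On restart it teleports the owner back to the saved location and rotation, then clears linear and angular physics velocities if the owner is a StaticMeshActor.
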(event Custom|OnGameRestart_Event
  (bind _returnvalue (Components|GetOwner))
  (bind _transform (Variables|Default|GetTransform))
  (Transformation|SetActorLocation _returnvalue (.location _transform) false true)
  (Transformation|SetActorRotation _returnvalue (.rotation _transform) true)
  (bind _asstatic_mesh_actor (Utilities|Casting|CastToStaticMeshActor (Components|GetOwner)))
  (Class|PrimitiveComponent|SetAllPhysicsLinearVelocity (Variables|/Script/Engine.StaticMeshActor|GetStaticMeshComponent _asstatic_mesh_actor) "0, 0, 0" false)
  (Class|PrimitiveComponent|SetAllPhysicsAngularVelocityinRadians (Variables|/Script/Engine.StaticMeshActor|GetStaticMeshComponent _asstatic_mesh_actor) (Math|Vector|MakeVector 0.0 0.0 0.0) false))

(event EventBeginPlay
  (Variables|Default|SetTransform (Transformation|GetActorTransform (Components|GetOwner)))
  (bind _asbp_bread_game_state (Utilities|Casting|CastToBP_BreadGameState (Game|GetGameState)))
  (EventDispatchers|AssignOnGameRestart _asbp_bread_game_state (delegate Custom|OnGameRestart_Event)))

(event EventTick
  (params (DeltaSeconds :type Float%20%28single-precision%29)))