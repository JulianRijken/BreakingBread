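; Blueprint function library with shared helpers for reaching the Bread actor and ending a level.
; GetBread returns the reference cached on BP_BreadGameState, falling back to an actor search that caches the first BP_Bread found and printing errors on failure.
; IsBreadMoving compares that actor's velocity length against a small threshold.
; CallEnding forwards an unlock event to the game state's LevelHandler through OnLevelClear.
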(fn GetBread
  (bind _asbp_bread_game_state (Utilities|Casting|CastToBP_BreadGameState (Game|GetGameState))
    (:then
      (bind _bread (Variables|/Game/Game/Core/BP_BreadGameState.BP_BreadGameState_C|GetBread _asbp_bread_game_state)
        (:then
          (return _bread))
        (:else
          (bind _outactors (Actor|GetAllActorsOfClass 0 "/Game/Game/Blueprint/BP_Bread.BP_Bread_C"))
          (Utilities|IsValid (Utilities|Array|Get(acopy) _outactors)
            (:Is%20Valid
              (bind _output_get (Variables|/Game/Game/Core/BP_BreadGameState.BP_BreadGameState_C|SetBread _asbp_bread_game_state (Utilities|Array|Get(acopy) _outactors)))
              (return _output_get))
            (:Is%20Not%20Valid
              (Development|PrintString 0 "ERROR Getting Bread" true true "(R=1.000000,G=0.038797,B=0.000000,A=1.000000)"))))))
    (:CastFailed
      (Development|PrintString 0 "ERROR Getting BreadMode" true true "(R=1.000000,G=0.136515,B=0.000000,A=1.000000)"))))

(fn IsBreadMoving
  (return (> (Math|Vector|VectorLength (Transformation|GetVelocity (CallFunction|GetBread))) 1e+01)))

(fn CallEnding
  (params (Unlock%20Event :type EUnlockEvents%20Enum :default "VE_NormalEnding"))
  (bind _asbp_bread_game_state (Utilities|Casting|CastToBP_BreadGameState (Game|GetGameState)))
  (Default|OnLevelClear (Variables|/Game/Game/Core/BP_BreadGameState.BP_BreadGameState_C|GetLevelHandler _asbp_bread_game_state) Unlock%20Event))