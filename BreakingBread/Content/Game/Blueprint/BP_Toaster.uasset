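; Toaster that launches the bread and triggers the toaster ending.
; Overlapping the box plays a timeline that pushes the button between two positions, and leaving it reverses the motion.
; Tick accumulates toasting time while the button is fully pressed, then fires the bread upward once past the limit.
; After launch, with the button no longer fully pressed, the ending is called once the bread's upward speed drops low.
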(event OnComponentBeginOverlap(Box)
  (params (OverlappedComponent :type Primitive%20Component%20Object%20Reference) (OtherActor :type Actor%20Object%20Reference) (OtherComp :type Primitive%20Component%20Object%20Reference) (OtherBodyIndex :type Integer) (bFromSweep :type Boolean) (SweepResult :type Hit%20Result%20Structure%20%28by%20ref%29))
  (bind _track (Timeline|Timeline Play)
    (:Update
      (Transformation|SetRelativeLocation (Variables|Default|GetSM_Button) (Math|Vector|Lerp(Vector) (Variables|Default|GetFrom) (Variables|Default|GetTo) _track) false false))))

(event OnComponentEndOverlap(Box)
  (params (OverlappedComponent :type Primitive%20Component%20Object%20Reference) (OtherActor :type Actor%20Object%20Reference) (OtherComp :type Primitive%20Component%20Object%20Reference) (OtherBodyIndex :type Integer))
  (bind _track (Timeline|Timeline Reverse)
    (:Update
      (Transformation|SetRelativeLocation (Variables|Default|GetSM_Button) (Math|Vector|Lerp(Vector) (Variables|Default|GetFrom) (Variables|Default|GetTo) _track) false false))))

(event EventBeginPlay
  (bind _timeline (Variables|Default|GetTimeline))
  (Components|Timeline|SetPlayRate _timeline (Variables|Default|GetSpeed))
  (Components|Timeline|SetNewTime _timeline 0.0))

(event EventTick
  (params (DeltaSeconds :type Float%20%28single-precision%29))
  (CallFunction|ToastN'Launch DeltaSeconds))

(fn ConstructionScript)

(fn ToastN'Launch
  (params (B :type Float%20%28double-precision%29))
  (if (== (Components|Timeline|GetPlaybackPosition (Variables|Default|GetTimeline)) 1.0)
    (bind _output_get (Variables|Default|SetElapsedSecondsToasting (+ (Variables|Default|GetElapsedSecondsToasting) B)))
    (if (< (Variables|Default|GetMaximalElapsedSecondsToasting) _output_get)
      (Physics|SetPhysicsLinearVelocity (Variables|/Script/Engine.SkeletalMeshActor|GetSkeletalMeshComponent (CallFunction|GetBread)) "0.000000,0.000000,1000.000000" false "None")
      (Default|SetToasted (CallFunction|GetBread) false)
      (Variables|Default|SetHasBeenLaunched true))
    (else
      (Variables|Default|SetElapsedSecondsToasting 0.0)
      (if (and (<= (.z (Transformation|GetVelocity (CallFunction|GetBread))) 1e+02) (Variables|Default|GetHasBeenLaunched))
        (CallFunction|CallEnding "VE_ToasterEnding")))))