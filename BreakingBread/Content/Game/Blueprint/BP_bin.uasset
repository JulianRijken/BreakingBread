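; Pedal bin that opens when the bread (BP_Bread) stands on its foot trigger and fires the GTA ending if the bread stays inside.
; Tick ramps a clamped alpha up or down to lerp lid and pedal rotation, with thresholds gating open and close sounds so they don't repeat.
; A second collider times the bread's stay, calling the ending after a short delay and printing debug messages.
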(event OnComponentBeginOverlap(FootTrigger)
  (params (OverlappedComponent :type Primitive%20Component%20Object%20Reference) (OtherActor :type Actor%20Object%20Reference) (OtherComp :type Primitive%20Component%20Object%20Reference) (OtherBodyIndex :type Integer) (bFromSweep :type Boolean) (SweepResult :type Hit%20Result%20Structure%20%28by%20ref%29))
  ;[1 1 1] Foot Collider
  (Utilities|Casting|CastToBP_Bread OtherActor)
  (Variables|Default|SetOverlapping true)
  ;;[1 1 1] Play Open Sound
  (if (<= (Variables|Default|GetAccumulatedTime) 0.1)
    (Audio|PlaySound2D "/Game/Game/Audio/TrashCanOpenCue.TrashCanOpenCue" 1.0 1.0 0.0 0 0)))

(event OnComponentEndOverlap(FootTrigger)
  (params (OverlappedComponent :type Primitive%20Component%20Object%20Reference) (OtherActor :type Actor%20Object%20Reference) (OtherComp :type Primitive%20Component%20Object%20Reference) (OtherBodyIndex :type Integer))
  ;[1 1 1] Foot Collider
  (Utilities|Casting|CastToBP_Bread OtherActor)
  (Variables|Default|SetOverlapping false))

(event OnComponentBeginOverlap(EndingCollider)
  (params (OverlappedComponent :type Primitive%20Component%20Object%20Reference) (OtherActor :type Actor%20Object%20Reference) (OtherComp :type Primitive%20Component%20Object%20Reference) (OtherBodyIndex :type Integer) (bFromSweep :type Boolean) (SweepResult :type Hit%20Result%20Structure%20%28by%20ref%29))
  (Utilities|Casting|CastToBP_Bread OtherActor)
  (Variables|Default|SetIsInsideBin true)
  (Development|PrintString "Bread in bin" true false))

(event OnComponentEndOverlap(EndingCollider)
  (params (OverlappedComponent :type Primitive%20Component%20Object%20Reference) (OtherActor :type Actor%20Object%20Reference) (OtherComp :type Primitive%20Component%20Object%20Reference) (OtherBodyIndex :type Integer))
  (Utilities|Casting|CastToBP_Bread OtherActor)
  (Variables|Default|SetIsInsideBin false)
  (Variables|Default|SetTimeInsidebin 0.0)
  (Development|PrintString "Bread Not in bin" true false))

(event EventTick
  (params (DeltaSeconds :type Float%20%28single-precision%29))
  (Utilities|FlowControl|Sequence
    (:then_0
      (if (Variables|Default|GetOverlapping)
        ;[1 1 1] Add Time
        (Variables|Default|SetAccumulatedTime (Math|Float|Clamp(Float) (+ (Variables|Default|GetAccumulatedTime) (/ DeltaSeconds (Variables|Default|GetTimeToOpen)))))
        (else
          ;[1 1 1] Substract Time
          (Variables|Default|SetAccumulatedTime (Math|Float|Clamp(Float) (+ (Variables|Default|GetAccumulatedTime) (/ (* DeltaSeconds -1.0) (Variables|Default|GetTimeToOpen)))))))
      (Utilities|FlowControl|Sequence
        (:then_0
          (Transformation|SetRelativeRotation (Variables|Default|Getlid) (Math|Rotator|Lerp(Rotator) "0, 0, 0" (Variables|Default|GetOpenpos) (Variables|Default|GetAccumulatedTime)) false false))
        (:then_1
          (Transformation|SetRelativeRotation (Variables|Default|Getfoot) (Math|Rotator|Lerp(Rotator) "0.000000,0.000000,-10.000000" "0.000000,0.000000,5.000000" (Variables|Default|GetAccumulatedTime)) false false))))
    (:then_1
      ;[1 1 1] Play Close Sound When needed
      (if (<= (Variables|Default|GetAccumulatedTime) 0.05)
        (if (not (Variables|Default|GetPlayedCloseSound))
          (Variables|Default|SetPlayedCloseSound true)
          (Audio|PlaySound2D "/Game/Game/Audio/TrashCanCloseCue.TrashCanCloseCue" 1.0 1.0 0.0 0 0))))
    (:then_2
      ;[1 1 1] Reset Played Close Sound
      (if (>= (Variables|Default|GetAccumulatedTime) 0.3)
        (Variables|Default|SetPlayedCloseSound false)))
    (:then_3
      (if (Variables|Default|GetIsInsideBin)
        (Development|PrintString (Utilities|String|Append "BREAD IS IN THE FREAKING FOR: " (Utilities|String|ToString(Float) (Variables|Default|GetTimeInsidebin))) true false "(R=0.045263,G=1.000000,B=0.000000,A=1.000000)")
        (bind _output_get (Variables|Default|SetTimeInsidebin (+ DeltaSeconds (Variables|Default|GetTimeInsidebin))))
        (if (>= _output_get 1.5)
          (CallFunction|CallEnding "VE_GTAEnding"))))))

(fn ConstructionScript)