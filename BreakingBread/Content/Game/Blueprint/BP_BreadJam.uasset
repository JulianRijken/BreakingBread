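; BP_BreadJam is an actor that triggers the relationship ending when bread comes to rest close to it.
; Each tick it takes the first BP_Bread overlapping its Box and checks its distance to the mesh, plus whether the bread is laying and not moving.
; A timer accumulates while these hold, resets if they fail during overlap, and calls the ending at a threshold, with on-screen debug prints.
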(event EventTick
  (params (DeltaSeconds :type Float%20%28single-precision%29))
  (bind _box (Variables|Default|GetBox))
  (bind _overlappingactors (Collision|GetOverlappingActors _box "/Game/Game/Blueprint/BP_Bread.BP_Bread_C" :!class /Script/Engine.PrimitiveComponent))
  (if (Math|Conversions|ToBoolean(Integer) (Utilities|Array|Length _overlappingactors))
    (if (Math|Boolean|ANDBoolean (<= (Math|Vector|Distance(Vector) (Transformation|GetActorLocation (Utilities|Array|Get(acopy) _overlappingactors)) (Transformation|GetWorldLocation (Variables|Debug|GetStaticMeshComponent))) (Variables|Default|GetMaximalDistance)) (Default|IsLaying (CallFunction|GetBread)) (not (CallFunction|IsBreadMoving)))
      (bind _output_get (Variables|Default|SetElapsedSeconds (+ (Variables|Default|GetElapsedSeconds) DeltaSeconds)))
      (Development|PrintString "Checking Relationship Ending" true true "(R=0.000000,G=1.000000,B=0.160000,A=1.000000)" 0.0)
      (if (>= _output_get (Variables|Default|GetMaximalElapsedSeconds))
        (Development|PrintString "Relationship Ending" true true "(R=1.000000,G=1.000000,B=0.000000,A=1.000000)" 0.0)
        (CallFunction|CallEnding "VE_RelationShipEnding"))
      (else
        (Variables|Default|SetElapsedSeconds 0.0)))))

(fn ConstructionScript)