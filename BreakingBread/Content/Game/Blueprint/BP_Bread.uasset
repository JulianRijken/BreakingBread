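; Grabbable physics bread actor that tracks its travel while not held and whether it is standing or laying.
; Tick applies custom gravity for normal, underwater or space states to the skeletal mesh and caps velocity by tutorial stage, which the NormalEnding unlock advances.
; Impacts while moving trigger debounced sound and particle bursts.
; Exposes teleport, reset to start, constraint-based movement locking and toasted material switching.
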(event OnComponentHit(SkeletalMeshComponent)
  (params (HitComponent :type Primitive%20Component%20Object%20Reference) (OtherActor :type Actor%20Object%20Reference) (OtherComp :type Primitive%20Component%20Object%20Reference) (NormalImpulse :type Vector :default "0, 0, 0") (Hit :type Hit%20Result%20Structure%20%28by%20ref%29))
  (if (CallFunction|IsBreadMoving)
    (Utilities|FlowControl|DoOnce false :!label _label
      (:Completed
        (Utilities|FlowControl|Sequence
          (:then_0
            (Utilities|FlowControl|Delay 0.2)
            (goto _label Reset))
          (:then_1
            (Audio|PlaySound2D "/Game/Game/Audio/BreadHit.BreadHit" 0.3 1.0 0.0 0 0)
            (Niagara|SpawnSystematLocation "/Game/Game/Art/FX/TestBurst.TestBurst" (Transformation|GetActorLocation) (Transformation|GetActorRotation))))))))

(event Custom|OnEndingUnlocked_Event
  (params (Unlock :type EUnlockEvents%20Enum :default "VE_NormalEnding"))
  (if (Utilities|Enum|Equal(Enum) Unlock "VE_NormalEnding")
    (Variables|Default|SetTutorialState 1)))

(event EventBeginPlay
  (Utilities|FlowControl|Sequence
    (:then_0
      (Variables|Default|SetStartPos (Transformation|GetActorLocation))
      (Variables|Default|SetStartEnd (Transformation|GetActorRotation)))
    (:then_2
      (bind _asbp_bread_game_state (Utilities|Casting|CastToBP_BreadGameState (Game|GetGameState)))
      (EventDispatchers|AssignOnEndingUnlocked _asbp_bread_game_state (delegate Custom|OnEndingUnlocked_Event)))))

(event Collision|EventActorBeginOverlap
  (params (OtherActor :type Actor%20Object%20Reference)))

(event EventTick
  (params (DeltaSeconds :type Float%20%28single-precision%29))
  (bind _returnvalue (Transformation|GetVelocity))
  (bind _max_velocity_tutorial (Variables|Default|GetMax%20Velocity%20Tutorial))
  (bind _tutorialstate (Variables|Default|GetTutorialState))
  (bind _maxvelocity (Variables|Default|GetMaxVelocity))
  (bind _returnvalue_2 (Math|Vector|VectorLength _returnvalue))
  (bind _returnvalue_3 (== _tutorialstate 0))
  (bind _returnvalue_4 (Math|Float|SelectFloat _max_velocity_tutorial _maxvelocity _returnvalue_3))
  (Utilities|FlowControl|Sequence
    (:then_0
      (if (not (Variables|Default|GetbIsGrabbed))
        (if (> _returnvalue_2 5.0)
          (Variables|Default|SetDistanceMoved (+ (Variables|Default|GetDistanceMoved) _returnvalue_2)))))
    (:then_1
      (Variables|Default|SetbIsLaying (< (Math|Float|Absolute(Float) (Math|Vector|DotProduct (Math|Vector|GetForwardVector (Transformation|GetActorRotation)) (Class|KismetMathLibrary|VectorForward))) (- 1.0 (Variables|Default|GetMinAmmountForDirection))))
      (Variables|Default|SetbIsStanding (> (Math|Float|Absolute(Float) (Math|Vector|DotProduct (Math|Vector|GetUpVector (Transformation|GetActorRotation)) (Math|Vector|VectorUp))) (Variables|Default|GetMinAmmountForDirection))))
    (:then_2
      (Class|PrimitiveComponent|SetAllPhysicsLinearVelocity (Variables|SkeletalMeshActor|GetSkeletalMeshComponent) (Math|Vector|MakeVector 0.0 0.0 (* (Variables|Default|GetGravityScale) -981.0 (Utilities|Time|GetWorldDeltaSeconds))) true))
    (:then_3
      (if (> (Math|Vector|VectorLength (Transformation|GetComponentVelocity (Variables|SkeletalMeshActor|GetSkeletalMeshComponent))) _returnvalue_4)
        (Class|PrimitiveComponent|SetAllPhysicsLinearVelocity (Variables|SkeletalMeshActor|GetSkeletalMeshComponent) (* (Math|Vector|Normalize (Transformation|GetComponentVelocity (Variables|SkeletalMeshActor|GetSkeletalMeshComponent))) _returnvalue_4) false)))
    (:then_5
      (if (Variables|Default|GetbInSpace)
        (Variables|Default|SetGravityScale 0.0)
        (elif (Variables|Default|GetbIsUnderWater)
          (Variables|Default|SetGravityScale (Variables|Default|GetWaterGravity))
          (else
            (Variables|Default|SetGravityScale (Variables|Default|GetNormalGravity))))))
    (:then_6
      (if (Variables|Default|GetbIsUnderWater)
        (Class|PrimitiveComponent|SetAllPhysicsLinearVelocity (Variables|SkeletalMeshActor|GetSkeletalMeshComponent) (Transformation|GetComponentVelocity (Variables|SkeletalMeshActor|GetSkeletalMeshComponent)) false)))))

(event EventOnPress)

(event EventOnRelease
  (Variables|Default|SetbIsGrabbed false))

(event EventOnGrab
  (Variables|Default|SetbIsGrabbed true))

(fn ConstructionScript)

(fn GetDistanceMoved
  (return (Variables|Default|GetDistanceMoved)))

(fn Teleport
  (params (Position :type Vector) (Rotation :type Rotator) (Keep%20Velocity :type Boolean))
  (Development|PrintString "Bread Teleported" true true "(R=1.000000,G=0.059748,B=0.019947,A=1.000000)")
  (Transformation|SetActorLocation Position false true)
  (Transformation|SetActorRotation Rotation true)
  (if (not Keep%20Velocity)
    (Class|PrimitiveComponent|SetAllPhysicsLinearVelocity (Variables|SkeletalMeshActor|GetSkeletalMeshComponent) "0, 0, 0" false)
    (Class|PrimitiveComponent|SetAllPhysicsAngularVelocityinRadians (Variables|SkeletalMeshActor|GetSkeletalMeshComponent) (Math|Vector|MakeVector 0.0 0.0 0.0) false)))

(fn IsStanding
  (return (Variables|Default|GetbIsStanding)))

(fn IsLaying
  (return (Variables|Default|GetbIsLaying)))

(fn IsGrabbed
  (return (Variables|Default|GetbIsGrabbed)))

(fn LockMovement
  (params (Lock :type Boolean))
  (if Lock
    (Class|PrimitiveComponent|SetConstraintMode (Variables|SkeletalMeshActor|GetSkeletalMeshComponent) "XYPlane")
    (elif (== (CallFunction|GetTutorialState) 0)
      (Class|PrimitiveComponent|SetConstraintMode (Variables|SkeletalMeshActor|GetSkeletalMeshComponent) "Default")
      (else
        (Class|PrimitiveComponent|SetConstraintMode (Variables|SkeletalMeshActor|GetSkeletalMeshComponent) "None")))))

(fn Reset
  (CallFunction|Teleport (Variables|Default|GetStartPos) (Variables|Default|GetStartEnd) false)
  (Variables|Default|SetDistanceMoved 0.0)
  (CallFunction|LockMovement true)
  (Development|PrintString "Bread Reset" true true "(R=1.000000,G=0.058055,B=0.000000,A=1.000000)"))

(fn SetUnderWater
  (params (UnderWater :type Boolean))
  (Variables|Default|SetbIsUnderWater UnderWater))

(fn SetinSpace
  (params (bInSpace :type Boolean))
  (Variables|Default|SetbInSpace bInSpace))

(fn SetToasted
  (params (bToasted :type Boolean))
  (bind _output_get (Variables|Default|SetbToasted bToasted))
  (Rendering|Material|SetMaterial (Variables|SkeletalMeshActor|GetSkeletalMeshComponent) 0 (select _output_get (Variables|Default|GetNormalMaterial) (Variables|Default|GetToastedMaterial)))
  (if (not _output_get)
    (Audio|PlaySoundatLocation (Variables|Default|GetSizzleSound) (Transformation|GetActorLocation) "0, 0, 0" 1.0 1.0 0.0 0 0 0 0)))

(fn IsToasted
  (return (Variables|Default|GetbToasted)))

(fn GetTutorialState
  (return (Variables|Default|GetTutorialState)))