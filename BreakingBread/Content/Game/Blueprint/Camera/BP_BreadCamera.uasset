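; Player camera pawn that orbits and zooms a cine camera around the bread and lets the mouse pick up and drag physics objects.
; It eases toward the bread's last position while nothing is grabbed, lerping focal length and spring-arm offset, with focus tracking the bread.
; Grabs use a trace and physics handle at fixed camera distance, notify BPI_Interact, and auto-release above max velocity.
; SetEnding blocks new grabs and reframes the shot.
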(event Input|EnhancedActionEvents|EnhancedInputActionIA_CameraLook
  (params (ActionValue :type Vector%202D%20Structure) (ElapsedSeconds :type Float%20%28double-precision%29) (TriggeredSeconds :type Float%20%28double-precision%29) (InputAction :type Input%20Action%20Object%20Reference :default "/Game/Game/Input/IA_CameraLook.IA_CameraLook"))
  (:Triggered
    (if (Variables|Default|GetRotateCamera)
      (Pawn|Input|AddControllerYawInput (.x ActionValue))
      (Pawn|Input|AddControllerPitchInput (.y ActionValue)))))

(event Input|EnhancedActionEvents|EnhancedInputActionIA_EnableLook
  (params (ActionValue :type Boolean) (ElapsedSeconds :type Float%20%28double-precision%29) (TriggeredSeconds :type Float%20%28double-precision%29) (InputAction :type Input%20Action%20Object%20Reference :default "/Game/Game/Input/IA_EnableLook.IA_EnableLook"))
  (:Started
    (bind _output_get (Variables|Default|SetRotateCamera ActionValue :!label _label))
    (Variables|/Script/Engine.PlayerController|SetCurrentMouseCursor (Game|GetPlayerController 0) (select _output_get "GrabHandClosed" "Hand")))
  (:Completed
    (goto _label)))

(event Input|EnhancedActionEvents|EnhancedInputActionIA_Grab
  (params (ActionValue :type Boolean) (ElapsedSeconds :type Float%20%28double-precision%29) (TriggeredSeconds :type Float%20%28double-precision%29) (InputAction :type Input%20Action%20Object%20Reference :default "/Game/Game/Input/IA_Grab.IA_Grab"))
  (:Started
    (if (not (Variables|Default|GetIsInEndng))
      (bind (_outhit _returnvalue) (Collision|LineTraceByChannel (Transformation|GetWorldLocation (Variables|Default|GetCineCamera)) (CallFunction|GetMouseWorldLocation) "TraceTypeQuery1" true 0 "ForDuration"))
      (if _returnvalue
        (if (Utilities|DoesObjectImplementInterface (.HitActor (Collision|BreakHitResult _outhit)) "/Game/Game/Blueprint/Camera/BPI_Interact.BPI_Interact_C")
          (Class|BPIInteract|OnPress(Message) (.HitActor (Collision|BreakHitResult _outhit))))
        (if (Physics|IsSimulatingPhysics (.HitComponent (Collision|BreakHitResult _outhit)) "None")
          (Variables|Default|SetGrabDistance (.Distance (Collision|BreakHitResult _outhit)))
          (Class|PhysicsHandleComponent|GrabComponentatLocation (Variables|Default|GetPhysicsHandle) (.HitComponent (Collision|BreakHitResult _outhit)) "None" (.ImpactPoint (Collision|BreakHitResult _outhit)))
          (Class|BPIInteract|OnGrab(Message) (.HitActor (Collision|BreakHitResult _outhit)))
          (bind _asbp_bread (Utilities|Casting|CastToBP_Bread (.HitActor (Collision|BreakHitResult _outhit))))
          (Default|ConstrainMovement _asbp_bread false)))))
  (:Completed
    (CallFunction|TryRelease)))

(event Input|EnhancedActionEvents|EnhancedInputActionIA_CameraZoom
  (params (ActionValue :type Float%20%28double-precision%29) (ElapsedSeconds :type Float%20%28double-precision%29) (TriggeredSeconds :type Float%20%28double-precision%29) (InputAction :type Input%20Action%20Object%20Reference :default "/Game/Game/Input/IA_CameraZoom.IA_CameraZoom"))
  (:Triggered
    (Variables|Default|SetTargetFocalLength (Math|Float|Clamp(Float) (+ (Variables|Default|GetTargetFocalLength) (* ActionValue (Variables|Default|GetZoomSpeed))) (Variables|Default|GetMinFocal) (Variables|Default|GetMaxFocal)))))

(event EventTick
  (params (DeltaSeconds :type Float%20%28single-precision%29))
  (bind _returnvalue (CallFunction|GetMouseWorldCameraPlaneConstrained))
  (bind _physicshandle (Variables|Default|GetPhysicsHandle))
  (bind _returnvalue_2 (Class|PhysicsHandleComponent|GetGrabbedComponent _physicshandle))
  (bind _returnvalue_3 (Transformation|GetComponentVelocity _returnvalue_2))
  (bind _returnvalue_4 (Math|Vector|VectorLength _returnvalue_3))
  ;[1 1 1] Tick
  (Utilities|FlowControl|Sequence
    (:then_0
      (Utilities|IsGrabbed
        (:true
          (Rendering|Debug|DrawDebugSphere _returnvalue 0.5 12 "(R=1.000000,G=0.000000,B=0.000000,A=1.000000)" 0.0 0.1)
          (Physics|Components|PhysicsHandle|SetTargetLocation (Variables|Default|GetPhysicsHandle) _returnvalue))))
    (:then_1
      (Utilities|IsGrabbed
        (:false
          (Variables|Default|SetTargetLastLocation (Transformation|GetActorLocation (CallFunction|GetBread))))))
    (:then_2
      (Transformation|SetActorLocation (Math|Vector|Lerp(Vector) (Transformation|GetActorLocation) (Variables|Default|GetTargetLastLocation) (Math|Float|Clamp(Float) (* (Utilities|Time|GetWorldDeltaSeconds) (Variables|Default|GetCameraMoveSpeed)))) false true))
    (:then_3
      (Utilities|IsGrabbed
        (:true
          (if (> _returnvalue_4 (Variables|Default|GetMaxVelocity))
            (Development|PrintString (Utilities|String|ToString(Float) _returnvalue_4) true true "(R=1.000000,G=0.061523,B=0.000000,A=1.000000)")
            (CallFunction|TryRelease)))))
    (:then_4
      (Variables|/Script/CinematicCamera.CineCameraComponent|SetCurrentFocalLength (Variables|Default|GetCineCamera) (Math|Float|Lerp (Variables|/Script/CinematicCamera.CineCameraComponent|GetCurrentFocalLength (Variables|Default|GetCineCamera)) (Variables|Default|GetTargetFocalLength) (Math|Float|Clamp(Float) (* (Utilities|Time|GetWorldDeltaSeconds) (Variables|Default|GetCameraLerpSpeed))))))
    (:then_5
      (Variables|/Script/Engine.SpringArmComponent|SetTargetOffset (Variables|Default|GetSpringArm) (Math|Vector|MakeVector 0.0 0.0 (Math|Float|Lerp (.z (Variables|/Script/Engine.SpringArmComponent|GetTargetOffset (Variables|Default|GetSpringArm))) (Variables|Default|GetTargetSpringArmOffset) (Math|Float|Clamp(Float) (* (Utilities|Time|GetWorldDeltaSeconds) (Variables|Default|GetSpringArmOffsetLerpSpeed)))))))))

(event EventBeginPlay
  (bind _returnvalue (Game|GetPlayerCameraManager 0))
  (Utilities|FlowControl|Sequence
    (:then_0
      (bind _asbp_bread_controller (Utilities|Casting|CastToBP_BreadController (Game|GetPlayerController 0)))
      (Utilities|IsValid (PlayerController|LocalPlayerSubsystems|GetEnhancedInputLocalPlayerSubsystem _asbp_bread_controller)
        (:Is%20Valid
          (Input|AddMappingContext (PlayerController|LocalPlayerSubsystems|GetEnhancedInputLocalPlayerSubsystem _asbp_bread_controller) "/Game/Game/Input/IA_MappingContext.IA_MappingContext" 0 (Utilities|Struct|MakeModifyContextOptions true false)))))
    (:then_1
      (Variables|/Script/Engine.PlayerCameraManager|SetViewPitchMin _returnvalue -9e+01)
      (Variables|/Script/Engine.PlayerCameraManager|SetViewPitchMax _returnvalue 1.0))
    (:then_2
      (Pawn|Input|AddControllerYawInput -2e+01)
      (Pawn|Input|AddControllerPitchInput 1e+01)
      (Transformation|SetRelativeRotation (Variables|Default|GetSpringArm) (Pawn|GetControlRotation :!class /Script/Engine.Pawn) false false))
    (:then_4
      (Variables|/Script/Engine.PlayerController|SetbShowMouseCursor (Game|GetPlayerController 0) true))
    (:then_5
      (bind _output_get (Variables|/Script/CinematicCamera.CineCameraComponent|SetCurrentFocalLength (Variables|Default|GetCineCamera) (Math|Float|Lerp (Variables|Default|GetMinFocal) (Variables|Default|GetMaxFocal) 0.5)))
      (Variables|Default|SetTargetFocalLength _output_get))
    (:then_6
      (Variables|/Script/CinematicCamera.CineCameraComponent|SetFocusSettings (Variables|Default|GetCineCamera) (Utilities|Struct|MakeCameraFocusSettings "Tracking" 1e+05 (Utilities|Struct|MakeCameraTrackingFocusSettings (Utilities|ResolveSoftReference (CallFunction|GetBread)) "0.000000,0.000000,0.000000" false) true 8.0 0.0)))))

(event Collision|EventActorBeginOverlap
  (params (OtherActor :type Actor%20Object%20Reference)))

(fn ConstructionScript)

(fn GetMouseWorldLocation
  (bind _returnvalue (Game|GetPlayerController 0))
  (bind (_worldlocation _worlddirection) (Game|Player|ConvertMouseLocationToWorldSpace _returnvalue))
  (return (+ _worldlocation (* (* _worlddirection (/ (.Z (Class|KismetMathLibrary|BreakVector3f _worldlocation)) (.Z (Class|KismetMathLibrary|BreakVector3f _worlddirection)))) -1.0))))

(fn GetMouseWorldCameraPlaneConstrained
  (bind _returnvalue (Game|GetPlayerController 0))
  (bind _grabdistance (Variables|Default|GetGrabDistance))
  (bind _cinecamera (Variables|Default|GetCineCamera))
  (bind _worlddirection (Game|Player|ConvertMouseLocationToWorldSpace _returnvalue))
  (bind _returnvalue_2 (Transformation|GetWorldLocation _cinecamera))
  (bind _returnvalue_3 (* _worlddirection _grabdistance))
  (bind _returnvalue_4 (+ _returnvalue_2 _returnvalue_3))
  (bind (_x _y _z) (Class|KismetMathLibrary|BreakVector3f _returnvalue_4))
  (return (Math|Vector|MakeVector _x _y (Math|Float|Clamp(Float) _z 0.0 5e+03))))

(fn TryRelease
  (bind _physicshandle (Variables|Default|GetPhysicsHandle))
  (bind _returnvalue (Class|PhysicsHandleComponent|GetGrabbedComponent _physicshandle))
  (bind _returnvalue_2 (Components|GetOwner _returnvalue))
  (Utilities|IsValid _returnvalue
    (:Is%20Valid
      (if (Utilities|DoesObjectImplementInterface _returnvalue_2 "/Game/Game/Blueprint/Camera/BPI_Interact.BPI_Interact_C")
        (Class|BPIInteract|OnRelease(Message) _returnvalue_2))
      (Physics|Components|PhysicsHandle|ReleaseComponent (Variables|Default|GetPhysicsHandle)))))

(fn ForceTeleport
  (params (Position :type Vector) (Snap%20Camera :type Boolean))
  (bind _output_get (Variables|Default|SetTargetLastLocation Position))
  (if Snap%20Camera
    (Transformation|SetActorLocation _output_get false true)))

(fn SetEnding
  (params (InEnding :type Boolean))
  (bind _output_get (Variables|Default|SetIsInEndng InEnding))
  (if _output_get
    (Variables|Default|SetTargetSpringArmOffset -5.0)
    (Variables|Default|SetTargetFocalLength 15.0)
    (else
      (Variables|Default|SetTargetSpringArmOffset 3.0))))