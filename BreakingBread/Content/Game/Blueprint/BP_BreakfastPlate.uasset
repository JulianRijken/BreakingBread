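; Breakfast plate Blueprint that triggers one of two game endings based on the food resting on it.
; Each Tick, while the bread is released, motionless and overlapping OverlapSphere, it counts time toward an ending.
; Enough bacon and eggs in the sphere advance the Breakfast ending timer; otherwise the Plate ending timer runs, each resetting the other.
; Both share one time threshold and pause, without resetting, whenever the bread condition fails.
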(event EventTick
  (params (DeltaSeconds :type Float%20%28single-precision%29))
  (if (not (Default|IsGrabbed (CallFunction|GetBread)))
    (if (CallFunction|IsBreadonPlate)
      (bind _iscounting (CallFunction|CheckBreakfastEnding DeltaSeconds))
      (CallFunction|CheckPlateEnding _iscounting DeltaSeconds))))

(fn ConstructionScript)

(fn IsBreadonPlate
  (return (and (not (CallFunction|IsBreadMoving)) (Math|Conversions|ToBoolean(Integer) (Utilities|Array|Length (Collision|GetOverlappingActors (Variables|Default|GetOverlapSphere) "/Game/Game/Blueprint/BP_Bread.BP_Bread_C" :!class /Script/Engine.PrimitiveComponent))))))

(fn AreSidesonPlate
  (bind _overlapsphere (Variables|Default|GetOverlapSphere))
  (return (and (>= (Utilities|Array|Length (Collision|GetOverlappingActors _overlapsphere "/Game/Game/Blueprint/BP_Bacon.BP_Bacon_C" :!class /Script/Engine.PrimitiveComponent)) (Variables|Default|GetMinimalBaconAmount)) (>= (Utilities|Array|Length (Collision|GetOverlappingActors _overlapsphere "/Game/Game/Blueprint/BP_Egg.BP_Egg_C" :!class /Script/Engine.PrimitiveComponent)) (Variables|Default|GetMinimalEggAmount)))))

(fn CheckBreakfastEnding
  (params (DeltaSeconds :type Float%20%28double-precision%29))
  (bind _result (CallFunction|AreSidesonPlate))
  (if _result
    (bind _output_get (Variables|Default|SetElapsedSecondsBreakfastEnding (+ (Variables|Default|GetElapsedSecondsBreakfastEnding) DeltaSeconds)))
    (Development|PrintString "Checking Breakfast Ending" true true "(R=0.000000,G=1.000000,B=0.160000,A=1.000000)" 0.0)
    (if (>= _output_get (Variables|Default|GetMaximalElapsedSeconds))
      (CallFunction|CallEnding "VE_BreakfastEnding")
      (Development|PrintString "Breakfast Ending" true true "(R=1.000000,G=1.000000,B=0.000000,A=1.000000)" 0.0))
    (else
      (Variables|Default|SetElapsedSecondsBreakfastEnding 0.0)))
  (return _result))

(fn CheckPlateEnding
  (params (IsBreakfastEndingCounting :type Boolean) (DeltaSeconds :type Float%20%28double-precision%29))
  (if IsBreakfastEndingCounting
    (Variables|Default|SetElapsedSecondsPlateEnding 0.0)
    (else
      (bind _output_get (Variables|Default|SetElapsedSecondsPlateEnding (+ DeltaSeconds (Variables|Default|GetElapsedSecondsPlateEnding))))
      (Development|PrintString "Checking Plate Ending" true true "(R=0.000000,G=1.000000,B=0.160000,A=1.000000)" 0.0)
      (if (>= _output_get (Variables|Default|GetMaximalElapsedSeconds))
        (CallFunction|CallEnding "VE_PlateEnding")
        (Development|PrintString "Plate Ending" true true "(R=1.000000,G=1.000000,B=0.000000,A=1.000000)" 0.0)))))