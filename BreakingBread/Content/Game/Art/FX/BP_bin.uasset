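; BP_bin is a bin whose lid swings open and foot rotates while a BP_Bread actor overlaps its Box.
; Begin and end overlap events set the Overlapping flag and reset a shared timer.
; Tick lerps both rotations from that timer, with a much longer divisor for closing than opening.
; The lid and foot branches each add delta time, so the timer advances twice per frame.
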(event OnComponentBeginOverlap(Box)
  (params (OverlappedComponent :type Primitive%20Component%20Object%20Reference) (OtherActor :type Actor%20Object%20Reference) (OtherComp :type Primitive%20Component%20Object%20Reference) (OtherBodyIndex :type Integer) (bFromSweep :type Boolean) (SweepResult :type Hit%20Result%20Structure%20%28by%20ref%29))
  (Utilities|Casting|CastToBP_Bread OtherActor)
  (if (not (Variables|Default|GetOverlapping))
    (Variables|Default|SetOverlapping true)
    (Variables|Default|SetAccumulatedTime 0.0)))

(event OnComponentEndOverlap(Box)
  (params (OverlappedComponent :type Primitive%20Component%20Object%20Reference) (OtherActor :type Actor%20Object%20Reference) (OtherComp :type Primitive%20Component%20Object%20Reference) (OtherBodyIndex :type Integer))
  (Utilities|Casting|CastToBP_Bread OtherActor)
  (Variables|Default|SetOverlapping false)
  (Variables|Default|SetAccumulatedTime 0.0))

(event EventTick
  (params (DeltaSeconds :type Float%20%28single-precision%29))
  (Utilities|FlowControl|Sequence
    (:then_0
      ;[1 1 1] lid
      (if (Variables|Default|GetOverlapping)
        (bind _output_get (Variables|Default|SetAccumulatedTime (+ (Variables|Default|GetAccumulatedTime) DeltaSeconds)))
        (Transformation|SetRelativeRotation (Variables|Default|Getlid) (Math|Rotator|Lerp(Rotator) "0, 0, 0" (Variables|Default|GetOpenpos) (Math|Float|Min(Float) (/ _output_get 3.0) 1.0)) false false)
        (else
          (bind _output_get_2 (Variables|Default|SetAccumulatedTime (+ (Variables|Default|GetAccumulatedTime) DeltaSeconds)))
          (Transformation|SetRelativeRotation (Variables|Default|Getlid) (Math|Rotator|Lerp(Rotator) (Variables|Default|GetOpenpos) "0, 0, 0" (Math|Float|Min(Float) (/ _output_get_2 3e+01) 1.0)) false false))))
    (:then_1
      ;[1 1 1] foot
      (if (Variables|Default|GetOverlapping)
        (bind _output_get_3 (Variables|Default|SetAccumulatedTime (+ (Variables|Default|GetAccumulatedTime) DeltaSeconds)))
        (Transformation|SetRelativeRotation (Variables|Default|Getfoot) (Math|Rotator|Lerp(Rotator) "0.000000,0.000000,-90.000000" (Variables|Default|Getturn%20foot) (Math|Float|Min(Float) (/ _output_get_3 3.0) 1.0)) false false)
        (else
          (bind _output_get_4 (Variables|Default|SetAccumulatedTime (+ (Variables|Default|GetAccumulatedTime) DeltaSeconds)))
          (Transformation|SetRelativeRotation (Variables|Default|Getfoot) (Math|Rotator|Lerp(Rotator) (Variables|Default|Getturn%20foot) "0.000000,0.000000,-90.000000" (Math|Float|Min(Float) (/ _output_get_4 3e+01) 1.0)) false false))))))

(fn ConstructionScript)