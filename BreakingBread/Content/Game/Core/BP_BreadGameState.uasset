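; Game state for the bread game that handles reaching endings and unlocking the persistent levels tied to them.
; A first-time ending is recorded, shows its name on the end screen and fades out, then resets the bread and camera and fades in.
; For every cleared ending, matching DataTable rows have their streaming levels unloaded and reloaded.
; A helper teleports bread and camera together.
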(event Custom|OnLevelClear
  (params (Unlock%20Event :type EUnlockEvents%20Enum :default "VE_BroodInRooster"))
  (bind _endwidget (Variables|Default|GetEndWidget))
  (if (== (Utilities|Array|FindItem (Variables|Default|GetClearedEndings) Unlock%20Event) -1)
    (if (not (Variables|Default|GetIsMovingOnToNextLevel))
      (Variables|Default|SetIsMovingOnToNextLevel true)
      (Utilities|Array|Add (Variables|Default|GetClearedEndings) Unlock%20Event)
      ;[1 1 1] Add the meme screen and set the text
      (Default|SetText _endwidget (Utilities|Text|ToText(String) (Utilities|String|EnumtoString Unlock%20Event)))
      (Default|Show _endwidget)
      (bind _asbp_bread_camera (Utilities|Casting|CastToBP_BreadCamera (Game|Player|GetPlayerPawn 0)))
      (Default|SetEnding _asbp_bread_camera true)
      ;[1 1 1] Start Fade and Timer
      (CameraFades|StartCameraFade :self (Game|GetPlayerCameraManager 0) :ToAlpha 1.0 :Duration (Variables|Default|GetFadeTime) :bShouldFadeAudio true :bHoldWhenFinished true)
      ;;[1 1 1] Remove the meme Screen
      (Utilities|FlowControl|Delay (Variables|Default|GetFadeTime))
      (Utilities|FlowControl|Delay 0.2)
      (Default|Hide (Variables|Default|GetEndWidget))
      (for _array_element (Variables|Default|GetClearedEndings)
        (CallFunction|ShowPersitantLevels _array_element)
        (CallFunction|ResetBread)
        (bind _asbp_bread_camera_2 (Utilities|Casting|CastToBP_BreadCamera (Game|Player|GetPlayerPawn 0)))
        (Default|SetEnding _asbp_bread_camera_2 false)
        (Utilities|FlowControl|Delay 1.0)
        (CameraFades|StartCameraFade :self (Game|GetPlayerCameraManager 0) :FromAlpha 1.0 :Duration (Variables|Default|GetFadeTime) :bShouldFadeAudio true :bHoldWhenFinished true)
        (Utilities|FlowControl|Delay (Variables|Default|GetFadeTime))
        (Variables|Default|SetIsMovingOnToNextLevel false)))))

(event Custom|Show%20Persitant%20levels
  (params (Unlock%20Event :type Byte))
  (bind _datatable (Variables|Default|GetDataTable))
  ;[1 1 1] Go Over each row in the table
  (bind _outrownames (DataTable|GetDataTableRowNames _datatable))
  (for _array_element _outrownames
    (bind _returnvalue (Utilities|GetDataTableRow _datatable _array_element)
      (:then
        ;[1 1 1] If the despatched Event Type corresponds with the unlock event
        (if (== (Math|Conversions|ToInteger(Byte) (.UnlockedByKey (Utilities|Struct|BreakUnlockedLevel _returnvalue))) (Math|Conversions|ToInteger(Byte) Unlock%20Event))
          (bind _returnvalue_2 (Class|WorldTools|GetLevelName (.Level (Utilities|Struct|BreakUnlockedLevel _returnvalue))))
          (Utilities|IsValid (Class|GameplayStatics|GetStreamingLevel _returnvalue_2)
            (:Is%20Valid
              (Variables|/Script/Engine.LevelStreaming|SetbShouldBeLoaded (Class|GameplayStatics|GetStreamingLevel _returnvalue_2) true)
              (Variables|/Script/Engine.LevelStreaming|SetbShouldBeVisible (Class|GameplayStatics|GetStreamingLevel _returnvalue_2) true)
              (Class|GameplayStatics|UnloadStreamLevelbySoftObjectPtr (.Level (Utilities|Struct|BreakUnlockedLevel _returnvalue)) true)
              (Class|GameplayStatics|LoadStreamLevelbySoftObjectPtr (.Level (Utilities|Struct|BreakUnlockedLevel _returnvalue)) true true))
            (:Is%20Not%20Valid
              (Development|PrintString "Make Sure To Add level You Want To Spawn" true true "(R=1.000000,G=0.000000,B=0.000000,A=1.000000)" 1e+01))))))))

(event EventBeginPlay
  (bind _returnvalue (UserInterface|CreateWidget "/Game/Game/Art/endscreens/WBP_EndScreen.WBP_EndScreen_C" (Game|GetPlayerController 0)))
  (UserInterface|Viewport|AddtoViewport _returnvalue 0)
  (Variables|Default|SetEndWidget _returnvalue))

(fn ConstructionScript)

(fn TeleportBread
  (params (Position :type Vector) (Rotation :type Rotator) (TeleportPhysics :type Boolean) (SnapCamera :type Boolean))
  (Default|Teleport (CallFunction|GetBread) Position Rotation TeleportPhysics)
  (bind _asbp_bread_camera (Utilities|Casting|CastToBP_BreadCamera (Game|Player|GetPlayerPawn 0)))
  (Default|ForceTeleport _asbp_bread_camera Position SnapCamera))

(fn LoadOpenedLevels)

(fn ResetBread
  (Default|Reset (CallFunction|GetBread))
  (bind _asbp_bread_camera (Utilities|Casting|CastToBP_BreadCamera (Game|Player|GetPlayerPawn 0)))
  (Default|ForceTeleport _asbp_bread_camera (Transformation|GetActorLocation (CallFunction|GetBread)) true))