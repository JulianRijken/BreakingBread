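; BP_BreadController is the controller for the bread game, handling input setup and game restarts.
; On begin play it adds the Enhanced Input mapping context.
; The restart action casts the game state to BP_BreadGameState, resets the bread and calls its game restart function.
; A debug B key uses a flip-flop to toggle the bread's toasted state.
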(event Input|EnhancedActionEvents|EnhancedInputActionIA_Restart
  (params (ActionValue :type Boolean) (ElapsedSeconds :type Float%20%28double-precision%29) (TriggeredSeconds :type Float%20%28double-precision%29) (InputAction :type Input%20Action%20Object%20Reference :default "/Game/Game/Input/IA_Restart.IA_Restart"))
  (:Triggered
    (bind _asbp_bread_game_state (Utilities|Casting|CastToBP_BreadGameState (Game|GetGameState)))
    (Default|ResetBread _asbp_bread_game_state)
    (Default|CallOnGameRestart _asbp_bread_game_state)))

(event EventBeginPlay
  (bind _returnvalue (PlayerController|LocalPlayerSubsystems|GetEnhancedInputLocalPlayerSubsystem))
  (Utilities|IsValid _returnvalue
    (:Is%20Valid
      (Input|AddMappingContext _returnvalue "/Game/Game/Input/IA_MappingContext.IA_MappingContext" 0 "(bIgnoreAllPressedKeysUntilRelease=True,bForceImmediately=False)"))))

(event Input|KeyboardEvents|DebugKeyB
  (params (Key :type Key%20Structure :default "None") (ActionValue :type Input%20Action%20Value%20Structure))
  (:Pressed
    (bind _isa (Utilities|FlowControl|FlipFlop)
      (:A
        _)
      (:B
        _))
    (Default|SetToasted (CallFunction|GetBread) _isa)))

(fn ConstructionScript)