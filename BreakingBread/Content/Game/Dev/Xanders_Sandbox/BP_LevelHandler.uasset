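; BP_LevelHandler spawns a level's interactable objects from a data table when OnLevelClear fires.
; LoadInteractableObjects scans every row, matches on LevelID and spawns that row's class at its stored transform, ignoring collisions.
; OnLevelClear casts the game state to BP_BreadGameState but does not yet read a level ID from it, always loading level 0.
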(event Custom|OnLevelClear
  ;[1 1 1] Get The Game State and read the level ID
  (Utilities|Casting|CastToBP_BreadGameState (Game|GetGameState))
  (CallFunction|LoadInteractableObjects))

(fn ConstructionScript)

(fn LoadInteractableObjects
  (params (LevelID :type Integer))
  (bind _datatable (Variables|Default|GetDataTable))
  (bind _outrownames (DataTable|GetDataTableRowNames _datatable))
  (for _array_element _outrownames
    (bind _returnvalue (Utilities|GetDataTableRow _datatable _array_element)
      (:then
        (if (== (.LevelID (Utilities|Struct|BreakDS_ObjectSpawnWaves _returnvalue)) LevelID)
          (Game|SpawnActorfromClass (.InteractableObject (Utilities|Struct|BreakDS_ObjectSpawnWaves _returnvalue)) (.InteractableObjectTransform (Utilities|Struct|BreakDS_ObjectSpawnWaves _returnvalue)) "AlwaysSpawn" "MultiplyWithRoot" 0 0))))))