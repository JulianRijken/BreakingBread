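; Dev bread slice actor that pairs a Chaos Flesh simulation with a skeletal mesh driven by a Deformer Graph.
; The construction script enables the Flesh component's simulation on the referenced Solver actor.
; Each Tick passes SimToRender and Amount to the mesh's Optimus deformer instance.
; Both deformer variable names are "None", so these writes target no named variable.
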(event EventBeginPlay)

(event Collision|EventActorBeginOverlap
  (params (OtherActor :type Actor%20Object%20Reference)))

(event EventTick
  (params (DeltaSeconds :type Float%20%28single-precision%29))
  (bind _asoptimus_deformer_instance (Utilities|Casting|CastToOptimusDeformerInstance (Variables|/Script/Engine.SkinnedMeshComponent|GetMeshDeformerInstance (Variables|SkeletalMeshActor|GetSkeletalMeshComponent))))
  (Class|OptimusDeformerInstance|SetTransformVariable _asoptimus_deformer_instance "None" (Variables|Default|GetSimToRender))
  (Class|OptimusDeformerInstance|SetFloatVariable _asoptimus_deformer_instance "None" (Variables|Default|GetAmount)))

(fn ConstructionScript
  (Class|DeformablePhysicsComponent|EnableSimulationfromActor (Variables|Default|GetFlesh) (Variables|Default|GetSolver)))